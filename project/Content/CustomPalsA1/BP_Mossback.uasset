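; Blueprint for the Mossback custom Pal that drives its visual mesh animations directly from code each Tick.
; A priority chain maps death, hit reactions, attacks, sleep, eating, roars, base work and movement speed to single animations played on MossbackVisual.
; A state integer and last-action reference prevent needless restarts while letting new actions retrigger one-shots.
; An HP drop also triggers a hit reaction, held for a few ticks before lower-priority states resume.
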(event EventTick
  (params (DeltaSeconds :type Float%20%28single-precision%29))
  (bind _returnvalue (Class|PalCharacter|GetActionComponent))
  (bind _returnvalue_2 (Class|PalCharacter|GetCharacterParameterComponent))
  (bind _returnvalue_3 (Class|PalCharacter|GetPalCharacterMovementComponent))
  (bind _mossbackvisual (Variables|Default|GetMossbackVisual))
  (bind _returnvalue_4 (Class|PalActionComponent|GetCurrentAction _returnvalue))
  (bind _returnvalue_5 (Class|PalCharacterMovementComponent|GetVelocity _returnvalue_3))
  (bind _returnvalue_6 (Class|PalCharacterParameterComponent|GetHP _returnvalue_2))
  (bind _returnvalue_7 (Math|Vector|VectorLengthXY _returnvalue_5))
  (bind _returnvalue_8 (Class|FixedPoint64MathLibrary|ConvertFixedPoint64toInt _returnvalue_6))
  (|CallParentFunction DeltaSeconds)
  (if (and (Utilities|IsValid _returnvalue) (Utilities|IsValid _returnvalue_2))
    (Variables|Default|SetA2HurtThisTick (< _returnvalue_8 (Variables|Default|GetA2LastHP)))
    (Variables|Default|SetA2LastHP _returnvalue_8)
    (Variables|Default|SetA2HoldTicks (Math|Integer|Max(Integer) (- (Variables|Default|GetA2HoldTicks) 1)))
    (if (or (Class|PalActionComponent|IsActiveActionType _returnvalue "Death" false) (Class|PalCharacterParameterComponent|IsDead _returnvalue_2))
      (if (!= (Variables|Default|GetA1State) 5)
        (Variables|Default|SetA1State 5)
        (Variables|Default|SetA1LastAction _returnvalue_4)
        (Variables|Default|SetA2HoldTicks 0)
        (Components|Animation|PlayAnimation _mossbackvisual "/Game/CustomPalsA1/AS_A2_Mossback_Faint.AS_A2_Mossback_Faint" false))
      (elif (or (or (or (or (Class|PalActionComponent|IsActiveActionType _returnvalue "Stan" false) (Class|PalActionComponent|IsActiveActionType _returnvalue "KnockBack" false)) (Class|PalActionComponent|IsActiveActionType _returnvalue "BlowAway" false)) (Class|PalActionComponent|IsActiveActionType _returnvalue "ElectricShock" false)) (Variables|Default|GetA2HurtThisTick))
        (if (or (or (!= (Variables|Default|GetA1State) 4) (!= _returnvalue_4 (Variables|Default|GetA1LastAction))) (Variables|Default|GetA2HurtThisTick))
          (Variables|Default|SetA1State 4)
          (Variables|Default|SetA1LastAction _returnvalue_4)
          (Variables|Default|SetA2HoldTicks 7)
          (Components|Animation|PlayAnimation _mossbackvisual "/Game/CustomPalsA1/AS_A2_Mossback_HitReact.AS_A2_Mossback_HitReact" false))
        (elif (not (> (Variables|Default|GetA2HoldTicks) 0))
          (if (or (or (Class|PalActionComponent|IsActiveActionType _returnvalue "GeneralAttack" false) (Class|PalActionComponent|IsActiveActionType _returnvalue "MeleeSkill" false)) (Class|PalActionComponent|IsActiveActionType _returnvalue "ShootSkill" false))
            (if (or (!= (Variables|Default|GetA1State) 3) (!= _returnvalue_4 (Variables|Default|GetA1LastAction)))
              (Variables|Default|SetA1State 3)
              (Variables|Default|SetA1LastAction _returnvalue_4)
              (Variables|Default|SetA2HoldTicks 0)
              (Components|Animation|PlayAnimation _mossbackvisual "/Game/CustomPalsA1/AS_Mossback_Attack.AS_Mossback_Attack" false))
            (elif (Class|PalActionComponent|IsActiveActionType _returnvalue "Sleep" false)
              (if (!= (Variables|Default|GetA1State) 6)
                (Variables|Default|SetA1State 6)
                (Variables|Default|SetA1LastAction _returnvalue_4)
                (Variables|Default|SetA2HoldTicks 0)
                (Components|Animation|PlayAnimation _mossbackvisual "/Game/CustomPalsA1/AS_A2_Mossback_Sleep.AS_A2_Mossback_Sleep" true))
              (elif (or (Class|PalActionComponent|IsActiveActionType _returnvalue "Eat" false) (Class|PalActionComponent|IsActiveActionType _returnvalue "HumanFeeding_DoMotion" false))
                (if (!= (Variables|Default|GetA1State) 7)
                  (Variables|Default|SetA1State 7)
                  (Variables|Default|SetA1LastAction _returnvalue_4)
                  (Variables|Default|SetA2HoldTicks 0)
                  (Components|Animation|PlayAnimation _mossbackvisual "/Game/CustomPalsA1/AS_A2_Mossback_Eat.AS_A2_Mossback_Eat" true))
                (elif (or (or (Class|PalActionComponent|IsActiveActionType _returnvalue "Menace" false) (Class|PalActionComponent|IsActiveActionType _returnvalue "Provocation" false)) (Class|PalActionComponent|IsActiveActionType _returnvalue "MimicryEncount" false))
                  (if (or (!= (Variables|Default|GetA1State) 8) (!= _returnvalue_4 (Variables|Default|GetA1LastAction)))
                    (Variables|Default|SetA1State 8)
                    (Variables|Default|SetA1LastAction _returnvalue_4)
                    (Variables|Default|SetA2HoldTicks 0)
                    (Components|Animation|PlayAnimation _mossbackvisual "/Game/CustomPalsA1/AS_A2_Mossback_Roar.AS_A2_Mossback_Roar" false))
                  (elif (or (or (or (or (or (or (or (or (or (or (or (or (or (or (or (or (or (Class|PalActionComponent|IsActiveActionType _returnvalue "CommonWork" false) (Class|PalActionComponent|IsActiveActionType _returnvalue "Architecture" false)) (Class|PalActionComponent|IsActiveActionType _returnvalue "Deforest" false)) (Class|PalActionComponent|IsActiveActionType _returnvalue "Mining" false)) (Class|PalActionComponent|IsActiveActionType _returnvalue "Feeding" false)) (Class|PalActionComponent|IsActiveActionType _returnvalue "GrowupPromotion" false)) (Class|PalActionComponent|IsActiveActionType _returnvalue "Watering" false)) (Class|PalActionComponent|IsActiveActionType _returnvalue "WateringOneshot" false)) (Class|PalActionComponent|IsActiveActionType _returnvalue "Harvest" false)) (Class|PalActionComponent|IsActiveActionType _returnvalue "GenerateEnergy" false)) (Class|PalActionComponent|IsActiveActionType _returnvalue "GenerateEnergyFire" false)) (Class|PalActionComponent|IsActiveActionType _returnvalue "GenerateEnergyElectric" false)) (Class|PalActionComponent|IsActiveActionType _returnvalue "Cooking" false)) (Class|PalActionComponent|IsActiveActionType _returnvalue "Ignition" false)) (Class|PalActionComponent|IsActiveActionType _returnvalue "Cool" false)) (Class|PalActionComponent|IsActiveActionType _returnvalue "SpawnItem" false)) (Class|PalActionComponent|IsActiveActionType _returnvalue "Resuscitation" false)) (Class|PalActionComponent|IsActiveActionType _returnvalue "DigOut" false))
                    (if (!= (Variables|Default|GetA1State) 9)
                      (Variables|Default|SetA1State 9)
                      (Variables|Default|SetA1LastAction _returnvalue_4)
                      (Variables|Default|SetA2HoldTicks 0)
                      (Components|Animation|PlayAnimation _mossbackvisual "/Game/CustomPalsA1/AS_A2_Mossback_WorkLoop.AS_A2_Mossback_WorkLoop" true))
                    (elif (> _returnvalue_7 1.8e+02)
                      (if (!= (Variables|Default|GetA1State) 2)
                        (Variables|Default|SetA1State 2)
                        (Variables|Default|SetA1LastAction _returnvalue_4)
                        (Variables|Default|SetA2HoldTicks 0)
                        (Components|Animation|PlayAnimation _mossbackvisual "/Game/CustomPalsA1/AS_Mossback_Run.AS_Mossback_Run" true))
                      (elif (> _returnvalue_7 8.0)
                        (if (!= (Variables|Default|GetA1State) 1)
                          (Variables|Default|SetA1State 1)
                          (Variables|Default|SetA1LastAction _returnvalue_4)
                          (Variables|Default|SetA2HoldTicks 0)
                          (Components|Animation|PlayAnimation _mossbackvisual "/Game/CustomPalsA1/AS_Mossback_Walk.AS_Mossback_Walk" true))
                        (elif (!= (Variables|Default|GetA1State) 0)
                          (Variables|Default|SetA1State 0)
                          (Variables|Default|SetA1LastAction _returnvalue_4)
                          (Variables|Default|SetA2HoldTicks 0)
                          (Components|Animation|PlayAnimation _mossbackvisual "/Game/CustomPalsA1/AS_Mossback_Idle.AS_Mossback_Idle" true))))))))))))))

(fn ConstructionScript
  (|CallParentFunction))