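; BP_Action_A_FungalHost is a custom Pal action that plays an attack montage on the acting character's main mesh.
; Beginning the action starts the montage and resets an elapsed timer, which each tick advances.
; It flags itself finished at a fixed time cap, or earlier if the montage stops after a short grace period.
; Both normal end and interruption stop the montage with a brief blend out.
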(event EventOnBeginAction
  (|CallParentFunction)
  (Animation|Montage|MontagePlay (Components|SkeletalMesh|GetAnimInstance (Class|PalCharacter|GetMainMesh (Class|PalActionBase|GetActionCharacter))) (Variables|Default|GetAttackMontage) 1.0 "MontageLength" 0.0 true)
  (Variables|Default|SetElapsed 0.0))

(event EventTickAction
  (params (DeltaTime :type Float%20%28single-precision%29))
  (|CallParentFunction DeltaTime)
  (Variables|Default|SetElapsed (+ (Variables|Default|GetElapsed) DeltaTime))
  (if (or (>= (Variables|Default|GetElapsed) 1.3199999999999998) (and (not (Animation|Montage|MontageIsPlaying (Components|SkeletalMesh|GetAnimInstance (Class|PalCharacter|GetMainMesh (Class|PalActionBase|GetActionCharacter))) (Variables|Default|GetAttackMontage))) (> (Variables|Default|GetElapsed) 0.1)))
    (Variables|Default|SetbIsEndAction true)))

(event EventOnEndAction
  (|CallParentFunction)
  (Animation|Montage|MontageStop (Components|SkeletalMesh|GetAnimInstance (Class|PalCharacter|GetMainMesh (Class|PalActionBase|GetActionCharacter))) 0.1 (Variables|Default|GetAttackMontage)))

(event EventOnBreakAction
  (|CallParentFunction)
  (Animation|Montage|MontageStop (Components|SkeletalMesh|GetAnimInstance (Class|PalCharacter|GetMainMesh (Class|PalActionBase|GetActionCharacter))) 0.1 (Variables|Default|GetAttackMontage)))