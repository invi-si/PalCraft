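; Redstone Revenant character Blueprint, apparently a custom Pal, that animates its emissive "A2Glow" material parameter in sync with attack and idle montages.
; Each Tick it checks the ChargeUp, Punch, SparkingIdle and ChargePunch montages in priority order and reads the playback position.
; Summed clamped linear ramps turn that position into a keyframed glow curve without curve assets, with a dim constant glow when none play.
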(event EventTick
  (params (DeltaSeconds :type Float%20%28single-precision%29))
  (bind _mesh (Variables|Character|GetMesh))
  (bind _returnvalue (Components|SkeletalMesh|GetAnimInstance _mesh))
  (bind _returnvalue_2 (Animation|Montage|MontageGetPosition _returnvalue "/Game/CustomPalsA1/AM_A2_RedstoneRevenant_ChargePunch.AM_A2_RedstoneRevenant_ChargePunch"))
  (bind _returnvalue_3 (Animation|Montage|MontageGetPosition _returnvalue "/Game/CustomPalsA1/AM_A2_RedstoneRevenant_ChargeUp.AM_A2_RedstoneRevenant_ChargeUp"))
  (bind _returnvalue_4 (Animation|Montage|MontageGetPosition _returnvalue "/Game/CustomPalsA1/AM_A2_RedstoneRevenant_Punch.AM_A2_RedstoneRevenant_Punch"))
  (bind _returnvalue_5 (Animation|Montage|MontageGetPosition _returnvalue "/Game/CustomPalsA1/AM_A2_RedstoneRevenant_SparkingIdle.AM_A2_RedstoneRevenant_SparkingIdle"))
  (|CallParentFunction DeltaSeconds)
  (if (Utilities|IsValid _returnvalue)
    (if (Animation|Montage|MontageIsPlaying _returnvalue "/Game/CustomPalsA1/AM_A2_RedstoneRevenant_ChargeUp.AM_A2_RedstoneRevenant_ChargeUp")
      (Rendering|Material|SetScalarParameterValueonMaterials _mesh "A2Glow" (+ (* (Math|Float|Clamp(Float) (/ (- _returnvalue_3 0.9333333333333333) 0.26666666666666666)) 0.0) (+ (* (Math|Float|Clamp(Float) (/ (- _returnvalue_3 0.8) 0.13333333333333333)) 5.1) (+ (* (Math|Float|Clamp(Float) (/ (- _returnvalue_3 0.6666666666666666) 0.13333333333333333)) -3.1) (+ (* (Math|Float|Clamp(Float) (/ (- _returnvalue_3 0.5666666666666667) 0.1)) 3.3) (+ (* (Math|Float|Clamp(Float) (/ (- _returnvalue_3 0.4666666666666667) 0.1)) -2.3) (+ (* (Math|Float|Clamp(Float) (/ (- _returnvalue_3 0.26666666666666666) 0.2)) 2.0) (+ (* (Math|Float|Clamp(Float) (/ (- _returnvalue_3 0.0) 0.26666666666666666)) 0.6) 0.4))))))))
      (elif (Animation|Montage|MontageIsPlaying _returnvalue "/Game/CustomPalsA1/AM_A2_RedstoneRevenant_Punch.AM_A2_RedstoneRevenant_Punch")
        (Rendering|Material|SetScalarParameterValueonMaterials _mesh "A2Glow" (+ (* (Math|Float|Clamp(Float) (/ (- _returnvalue_4 0.5333333333333333) 0.26666666666666666)) -0.6) (+ (* (Math|Float|Clamp(Float) (/ (- _returnvalue_4 0.3333333333333333) 0.2)) -3.0) (+ (* (Math|Float|Clamp(Float) (/ (- _returnvalue_4 0.23333333333333334) 0.1)) -4.0) (+ (* (Math|Float|Clamp(Float) (/ (- _returnvalue_4 0.13333333333333333) 0.1)) 3.0) (+ (* (Math|Float|Clamp(Float) (/ (- _returnvalue_4 0.0) 0.13333333333333333)) -1.0) 6.0))))))
        (elif (Animation|Montage|MontageIsPlaying _returnvalue "/Game/CustomPalsA1/AM_A2_RedstoneRevenant_SparkingIdle.AM_A2_RedstoneRevenant_SparkingIdle")
          (Rendering|Material|SetScalarParameterValueonMaterials _mesh "A2Glow" (+ (* (Math|Float|Clamp(Float) (/ (- _returnvalue_5 1.4) 0.6)) 0.0) (+ (* (Math|Float|Clamp(Float) (/ (- _returnvalue_5 1.3333333333333333) 0.06666666666666667)) -3.6) (+ (* (Math|Float|Clamp(Float) (/ (- _returnvalue_5 1.2666666666666666) 0.06666666666666667)) 3.6) (+ (* (Math|Float|Clamp(Float) (/ (- _returnvalue_5 0.6666666666666666) 0.6)) 0.0) (+ (* (Math|Float|Clamp(Float) (/ (- _returnvalue_5 0.6) 0.06666666666666667)) -4.6) (+ (* (Math|Float|Clamp(Float) (/ (- _returnvalue_5 0.5333333333333333) 0.06666666666666667)) 4.6) (+ (* (Math|Float|Clamp(Float) (/ (- _returnvalue_5 0.0) 0.5333333333333333)) 0.0) 0.4))))))))
          (elif (Animation|Montage|MontageIsPlaying _returnvalue "/Game/CustomPalsA1/AM_A2_RedstoneRevenant_ChargePunch.AM_A2_RedstoneRevenant_ChargePunch")
            (Rendering|Material|SetScalarParameterValueonMaterials _mesh "A2Glow" (+ (* (Math|Float|Clamp(Float) (/ (- _returnvalue_2 1.7333333333333334) 0.26666666666666666)) -0.6) (+ (* (Math|Float|Clamp(Float) (/ (- _returnvalue_2 1.5333333333333334) 0.2)) -3.0) (+ (* (Math|Float|Clamp(Float) (/ (- _returnvalue_2 1.4333333333333333) 0.1)) -4.0) (+ (* (Math|Float|Clamp(Float) (/ (- _returnvalue_2 1.3333333333333333) 0.1)) 3.0) (+ (* (Math|Float|Clamp(Float) (/ (- _returnvalue_2 1.2) 0.13333333333333333)) -1.0) (+ (* (Math|Float|Clamp(Float) (/ (- _returnvalue_2 0.9333333333333333) 0.26666666666666666)) 0.0) (+ (* (Math|Float|Clamp(Float) (/ (- _returnvalue_2 0.8) 0.13333333333333333)) 5.1) (+ (* (Math|Float|Clamp(Float) (/ (- _returnvalue_2 0.6666666666666666) 0.13333333333333333)) -3.1) (+ (* (Math|Float|Clamp(Float) (/ (- _returnvalue_2 0.5666666666666667) 0.1)) 3.3) (+ (* (Math|Float|Clamp(Float) (/ (- _returnvalue_2 0.4666666666666667) 0.1)) -2.3) (+ (* (Math|Float|Clamp(Float) (/ (- _returnvalue_2 0.26666666666666666) 0.2)) 2.0) (+ (* (Math|Float|Clamp(Float) (/ (- _returnvalue_2 0.0) 0.26666666666666666)) 0.6) 0.4)))))))))))))
            (else
              (Rendering|Material|SetScalarParameterValueonMaterials _mesh "A2Glow" 0.4))))))))

(fn ConstructionScript
  (|CallParentFunction))